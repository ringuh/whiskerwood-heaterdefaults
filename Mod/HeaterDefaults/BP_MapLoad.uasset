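; Mod actor for HeaterDefaults that applies a configured "Turn on at" temperature to newly built fueled heaters.
; On load it records existing Heaters and Bonfires as known without changing them.
; Building spawns are handled directly, while destroyed construction sites trigger timed rescans with limited retries to find new heaters.
; Eligible heaters receive the autopause limit through a UI_HeaterView widget's HUD action, reusing the game's UI logic.
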(event `self.ReceiveBeginPlay`
  (bind _returnvalue (`ModAPI.GetModAPI`))
  (add `ModAPI.onLoadingFinished` _returnvalue (delegate `OnLoaded`))
  (add `ModAPI.onConstructionSpawned` _returnvalue (delegate `OnConstruction`))
  (add `ModAPI.onBuildingSpawned` _returnvalue (delegate `OnBuilt`))
  (`ModAPI.LogMessage` (`ModAPI.GetModAPI`) "HeaterDefaults ready" true))

(event `OnLoaded`
  (bind _cur (`self.Cur`))
  (bind _retries (`self.Retries`))
  (bind _view (`self.View`))
  (bind _returnvalue (`self.GetComponentByClass` _cur "/Script/ProjectArco.FueledHeater"))
  (set `self.LoadScan` true)
  (set `self.SingleMode` false)
  (set `self.KnownBefore` (`KismetArrayLibrary.Array_Length` (`self.Known`)) :!label _label)
  (if (not (`KismetSystemLibrary.IsValid` (`self.View`)))
    (bind _returnvalue_2 (`|CreateWidget` "/Script/ProjectArco.UI_HeaterView" (`GameplayStatics.GetPlayerController` 0)))
    (set `self.View` _returnvalue_2))
  (bind _returnvalue_3 (`ModAPI.ReadModOptionValue` (`ModAPI.GetModAPI`) "HeaterDefaults_TurnOnAt" "0"))
  (bind _returnvalue_4 (`ModAPI.ReadDataTableValue` (`ModAPI.GetModAPI`) "SystemTunes" "HeatIncrementU8" "FloatValue"))
  (if (`self.SingleMode`)
    (set `self.Cur` (`self.Built`))
    (if (and (`KismetSystemLibrary.IsValid` _returnvalue) (not (`KismetArrayLibrary.Array_Contains` (`self.Known`) _cur))) :!label _label_2
      (`KismetArrayLibrary.Array_Add` (`self.Known`) _cur)
      (if (and (!= (`FueledHeater.m_fuelSource` _returnvalue) 2) (not (`self.LoadScan`)))
        (`KismetSystemLibrary.SetObjectPropertyByName` _view "Context" _cur)
        (bind _returnvalue_5 (`UI_HeaterView.CalcHudState` _view))
        (bind ((`maxTempToEnable_playerUnits` _maxtemptoenable_playerunits) (`allowReset` _allowreset)) (break `FueledHeaterHudInfo` _returnvalue_5))
        (bind _returnvalue_6 (`KismetStringLibrary.Conv_StringToInt` _returnvalue_3))
        (if (not (or _allowreset (== _maxtemptoenable_playerunits _returnvalue_6)))
          (bind _asgrid_actor (cast `GridActor` _cur))
          (bind _returnvalue_7 (`KismetMathLibrary.FTrunc` (+ (`KismetStringLibrary.Conv_StringToDouble` _returnvalue_4) 0.5)))
          (`ArcoWidgetBase.ReceiveHudAction` _view (make `HudAction` :`action` "setAutopauseLimit" :`paramInt` (+ (* (+ _returnvalue_6 30) 3) (`KismetMathLibrary.SelectInt` _returnvalue_7 15 (> _returnvalue_7 0))) :`paramGrid` (`.rootPosition` (break `GridFootprint` (`GridActor.liveFootprint` _asgrid_actor)))))
          (`ModAPI.LogMessage` (`ModAPI.GetModAPI`) (`KismetStringLibrary.Concat_StrStr` (`KismetStringLibrary.Concat_StrStr` (`KismetStringLibrary.Concat_StrStr` (`KismetStringLibrary.Concat_StrStr` (`KismetStringLibrary.Concat_StrStr` "HeaterDefaults: ") (`KismetSystemLibrary.GetDisplayName` _cur)) " Turn on at -> ") (`KismetStringLibrary.Conv_IntToString` _returnvalue_6)) " C") true))))
    (else
      (bind _outactors (`GameplayStatics.GetAllActorsOfClass` "/Game/GridActors/Heater.Heater_C"))
      (for _array_element _outactors
        (set `self.Cur` _array_element)
        (goto _label_2))
      (bind _outactors_2 (`GameplayStatics.GetAllActorsOfClass` "/Game/GridActors/bonfire.bonfire_C"))
      (for _array_element_2 _outactors_2
        (set `self.Cur` _array_element_2)
        (goto _label_2))
      (if (and (== (`KismetArrayLibrary.Array_Length` (`self.Known`)) (`self.KnownBefore`)) (> _retries 0))
        (set `self.Retries` (- _retries 1))
        (`KismetSystemLibrary.K2_SetTimer` self "OnScanTimer" 1.0)
        (else
          (set `self.Retries` 0))))))

(event `OnConstruction`
  (params (Actor :type "Actor Object Reference"))
  (add `self.OnDestroyed` Actor (delegate `OnSiteGone`)))

(event `OnSiteGone` :!signature `self.OnDestroyed`
  (params (DestroyedActor :type "Actor Object Reference"))
  (set `self.Retries` 3)
  (`KismetSystemLibrary.K2_SetTimer` self "OnScanTimer" 1.0))

(event `OnBuilt`
  (params (Actor :type "Actor Object Reference"))
  (if (`KismetSystemLibrary.IsValid` (`self.GetComponentByClass` Actor "/Script/ProjectArco.FueledHeater"))
    (set `self.Built` Actor)
    (set `self.LoadScan` false)
    (set `self.SingleMode` true)
    (goto _label)))

(event `OnScanTimer`
  (set `self.LoadScan` false)
  (set `self.SingleMode` false)
  (goto _label))

(fn `UserConstructionScript`)